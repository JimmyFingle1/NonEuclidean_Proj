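; BP_EfficientLoopingWorld is a spawner that builds a grid of looping world tiles when play begins.
; BeginPlay runs nested loops over grid width and height, spacing positions by tile size, and spawns a BP_LoopingObjectArray at each.
; Positions start at the world origin rather than the actor's location; any looping behaviour lives in the spawned actors, and an unused spawn node remains disconnected.
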(event EventBeginPlay
  (for _index (range 0 (- (Variables|Default|GetGridWidth) 1)) ; X
    (for _index_2 (range 0 (- (Variables|Default|GetGridHeight) 1)) ; Y
      (bind _output_get (Variables|Default|SetStartLocation (Math|Vector|MakeVector (Math|Conversions|ToFloat(Integer) (* _index (Variables|Default|GetTileSize))) (Math|Conversions|ToFloat(Integer) (* _index_2 (Variables|Default|GetTileSize))) 0.0))) ; Set start location
      (Game|SpawnActorfromClass "/Game/JPContent/BP_LoopingObjectArray.BP_LoopingObjectArray_C" (Math|Conversions|ToTransform(Vector) _output_get) "Undefined" "MultiplyWithRoot" 0 0))))

(fn ConstructionScript)