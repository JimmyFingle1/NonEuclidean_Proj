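; BP_Door is an interactable door that opens while enough pressure switches are active and closes otherwise.
; SwitchActivated and SwitchDeactivated events adjust an active-switch count and compare it to the required number.
; The DoorActive timeline plays or reverses to move the door mesh along relative Z.
; An open or close sound plays at the door on every switch change, even if the door's state is unchanged.
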(event Custom|SwitchActivated
  (Math|Integer|IncrementInt (Variables|Default|GetPressureSwitchesActive)
    (:%20%20
      (if (>= (Variables|Default|GetPressureSwitchesActive) (Variables|Default|GetPressureSwitchesNeeded))
        (Audio|PlaySoundatLocation "/Game/JPContent/Audio/MS_OpenDoor13D.MS_OpenDoor13D" (Transformation|GetWorldLocation (Variables|Default|GetDoor)) "0, 0, 0" 1.0 1.0 0.0 0 0 0 0)
        (bind _doorpos (Timeline|Door%20Active Play)
          (:Update
            (Transformation|SetRelativeLocation (Variables|Default|GetDoor) (Math|Vector|MakeVector 0.0 0.0 _doorpos) false false)))
        (else
          (Audio|PlaySoundatLocation "/Game/JPContent/Audio/MS_DoorClose.MS_DoorClose" (Transformation|GetWorldLocation (Variables|Default|GetDoor)) "0, 0, 0" 1.0 1.0 0.0 0 0 0 0)
          (Timeline|Door%20Active Reverse))))))

(event Custom|SwitchDeactivated
  (Math|Integer|DecrementInt (Variables|Default|GetPressureSwitchesActive)
    (:%20%20
      (if (>= (Variables|Default|GetPressureSwitchesActive) (Variables|Default|GetPressureSwitchesNeeded))
        (Audio|PlaySoundatLocation "/Game/JPContent/Audio/MS_OpenDoor13D.MS_OpenDoor13D" (Transformation|GetWorldLocation (Variables|Default|GetDoor)) "0, 0, 0" 1.0 1.0 0.0 0 0 0 0)
        (bind _doorpos (Timeline|Door%20Active Play)
          (:Update
            (Transformation|SetRelativeLocation (Variables|Default|GetDoor) (Math|Vector|MakeVector 0.0 0.0 _doorpos) false false)))
        (else
          (Audio|PlaySoundatLocation "/Game/JPContent/Audio/MS_DoorClose.MS_DoorClose" (Transformation|GetWorldLocation (Variables|Default|GetDoor)) "0, 0, 0" 1.0 1.0 0.0 0 0 0 0)
          (Timeline|Door%20Active Reverse))))))

(event EventBeginPlay)

(event Collision|EventActorBeginOverlap
  (params (OtherActor :type Actor%20Object%20Reference)))

(event EventTick
  (params (DeltaSeconds :type Float%20%28single-precision%29)))

(fn ConstructionScript)