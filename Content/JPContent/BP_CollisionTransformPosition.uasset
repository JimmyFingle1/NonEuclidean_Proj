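; BP_CollisionTransformPosition is a trigger box that toggles a referenced object's height when the Superliminal first-person character leaves it.
; On BeginPlay it caches the player character and snaps the first MoveObjects entry to StartZ, keeping X and Y.
; Each end overlap instantly switches that object between StartZ and NewZ based on its current Z.
; DestroyOnTrigger removes the trigger after a move to NewZ, making it one-shot.
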(event OnComponentEndOverlap(Box)
  (params (OverlappedComponent :type Primitive%20Component%20Object%20Reference) (OtherActor :type Actor%20Object%20Reference) (OtherComp :type Primitive%20Component%20Object%20Reference) (OtherBodyIndex :type Integer))
  (bind _move_objects (Variables|Default|GetMove%20Objects))
  (bind _move_objects_2 (Variables|Default|GetMove%20Objects))
  (bind _output (Utilities|Array|Get(acopy) _move_objects))
  (bind _output_2 (Utilities|Array|Get(acopy) _move_objects_2))
  (bind _rootcomponent (Variables|/Script/Engine.Actor|GetRootComponent _output))
  (bind _rootcomponent_2 (Variables|/Script/Engine.Actor|GetRootComponent _output_2))
  (bind _returnvalue (Transformation|GetWorldLocation _rootcomponent))
  (bind _returnvalue_2 (Transformation|GetWorldLocation _rootcomponent_2))
  (Utilities|Casting|CastToFPS_Superliminal OtherActor)
  (if (== (.z (.location (Transformation|GetWorldTransform (Variables|/Script/Engine.Actor|GetRootComponent (Utilities|Array|Get(acopy) (Variables|Default|GetMove%20Objects)))))) (Variables|Default|GetStartZ))
    (Transformation|SetWorldLocation _rootcomponent_2 (Math|Vector|MakeVector (.x _returnvalue_2) (.y _returnvalue_2) (Variables|Default|GetNewZ)) false false)
    (if (Variables|Default|GetDestroyOnTrigger)
      (Actor|DestroyActor))
    (else
      (Transformation|SetWorldLocation _rootcomponent (Math|Vector|MakeVector (.x _returnvalue) (.y _returnvalue) (Variables|Default|GetStartZ)) false false))))

(event EventBeginPlay
  (bind _move_objects (Variables|Default|GetMove%20Objects))
  (bind _output (Utilities|Array|Get(acopy) _move_objects))
  (bind _rootcomponent (Variables|/Script/Engine.Actor|GetRootComponent _output))
  (bind _returnvalue (Transformation|GetWorldLocation _rootcomponent))
  (bind _asfps_superliminal (Utilities|Casting|CastToFPS_Superliminal (Game|GetPlayerCharacter 0)))
  (Variables|Default|SetPC _asfps_superliminal)
  (Transformation|SetWorldLocation _rootcomponent (Math|Vector|MakeVector (.x _returnvalue) (.y _returnvalue) (Variables|Default|GetStartZ)) false false))

(event Collision|EventActorBeginOverlap
  (params (OtherActor :type Actor%20Object%20Reference)))

(event EventTick
  (params (DeltaSeconds :type Float%20%28single-precision%29)))

(fn ConstructionScript)