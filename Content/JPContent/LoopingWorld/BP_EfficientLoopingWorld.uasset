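; Actor Blueprint that builds the tiled grid for a looping world when play begins.
; Nested loops over grid width and length spawn a looping object tile and an other-looping-objects actor at each tile-spaced location.
; The inner loop also repeatedly moves the InfinateLoopTps actor to the grid's center at a set height.
; Disconnected leftover nodes hold a single tile spawn and a PlayerSpawn centering step.
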(event EventBeginPlay
  (Variables|Default|SetLooping%20object%20tile "/Game/JPContent/LoopingWorld/BP_LoopingObjectTile.BP_LoopingObjectTile_C")
  (Variables|Default|SetOther%20Looping%20Objects "/Game/JPContent/LoopingWorld/BP_OtherLoopingObjects.BP_OtherLoopingObjects_C")
  (for _index (range 0 (- (Variables|Default|GetGridWidth) 1)) ; X
    (for _index_2 (range 0 (- (Variables|Default|GetGridLength) 1)) ; Y
      (bind _output_get (Variables|Default|SetStartLocation (Math|Vector|MakeVector (Math|Conversions|ToFloat(Integer) (* _index (Variables|Default|GetTileSize))) (Math|Conversions|ToFloat(Integer) (* _index_2 (Variables|Default|GetTileSize))) 0.0))) ; Set start location
      (Game|SpawnActorfromClass (Variables|Default|GetLooping%20object%20tile) (Math|Conversions|ToTransform(Vector) _output_get) "Undefined" "MultiplyWithRoot" 0 0)
      (Game|SpawnActorfromClass (Variables|Default|GetOther%20Looping%20Objects) (Math|Conversions|ToTransform(Vector) _output_get) "Undefined" "MultiplyWithRoot" 0 0)
      (Transformation|SetActorTransform (Variables|Default|GetInfinateLoopTps) (Math|Transform|MakeTransform (Math|Vector|MakeVector (* (* (- (Variables|Default|GetGridWidth) 1) (Variables|Default|GetTileSize)) 0.5) (* (* (- (Variables|Default|GetGridLength) 1) (Variables|Default|GetTileSize)) 0.5) (Variables|Default|GetZPos)) "0, 0, 0" "1.000000,1.000000,1.000000")))))

(fn ConstructionScript)