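; BP_TeleporterActorCollection is a looping-world teleporter that moves Characters to a linked teleporter when they leave a trigger.
; End-overlap events on OuterTeleporter and OuterTeleporter1 target ConnectedTeleporter and ConnectedTeleporter1 respectively, behind a validity check.
; The destination keeps the character's offset from this actor, reapplied at the linked teleporter's location, with rotation unchanged.
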(event OnComponentEndOverlap(OuterTeleporter)
  (params (OverlappedComponent :type Primitive%20Component%20Object%20Reference) (OtherActor :type Actor%20Object%20Reference) (OtherComp :type Primitive%20Component%20Object%20Reference) (OtherBodyIndex :type Integer))
  ;[1 1 1] Get this for MPG
  (Utilities|Casting|CastToCharacter OtherActor)
  (Utilities|IsValid 0
    (:Is%20Valid
      (Transformation|Teleport OtherActor (- (Transformation|GetActorLocation (Variables|Default|GetConnectedTeleporter)) (- (Transformation|GetActorLocation self) (Transformation|GetActorLocation OtherActor))) (Transformation|GetActorRotation OtherActor)))))

(event OnComponentEndOverlap(OuterTeleporter1)
  (params (OverlappedComponent :type Primitive%20Component%20Object%20Reference) (OtherActor :type Actor%20Object%20Reference) (OtherComp :type Primitive%20Component%20Object%20Reference) (OtherBodyIndex :type Integer))
  ;[1 1 1] Get this for MPG
  (Utilities|Casting|CastToCharacter OtherActor)
  (Utilities|IsValid 0
    (:Is%20Valid
      (Transformation|Teleport OtherActor (- (Transformation|GetActorLocation (Variables|Default|GetConnectedTeleporter1)) (- (Transformation|GetActorLocation self) (Transformation|GetActorLocation OtherActor))) (Transformation|GetActorRotation OtherActor)))))

(fn ConstructionScript)